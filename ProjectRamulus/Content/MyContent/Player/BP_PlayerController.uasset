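; Player controller that sets up input and the menu UI for BP_Player.
; On possess it adds the default Enhanced Input mapping context, creates the main, pause and chapter menu widgets, stores them on the player, then shows the main menu.
; Pause and any-key input actions are forwarded to the player pawn.
; Mouse and gamepad input events are empty, and mouse cursor toggling is left unconnected.
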(event `self.ReceivePossess`
  (params (PossessedPawn :type "Pawn Object Reference"))
  (bind _asbp_player (cast `/Game/MyContent/Player/BP_Player` PossessedPawn))
  (set `self.PlayerRef` _asbp_player)
  (`self.DefaultInputs`)
  (`self.CreateWidgetRefs`)
  (`UserWidget.AddToViewport` (`/Game/MyContent/Player/BP_Player.MainMenuRef` (`self.PlayerRef`)) 0))

(event `EnhancedInput|/Game/MyContent/Player/Input/IA_Pause`
  (params (ActionValue :type Boolean) (ElapsedSeconds :type "Float (double-precision)") (TriggeredSeconds :type "Float (double-precision)") (InputAction :type "InputAction Object Reference" :default "/Game/MyContent/Player/Input/IA_Pause.IA_Pause"))
  (:`Triggered`
    (`/Game/MyContent/Player/BP_Player.PauseMenu` (`self.PlayerRef`))))

(event `EnhancedInput|/Game/MyContent/Player/Input/IA_AnyKey`
  (params (ActionValue :type Boolean) (ElapsedSeconds :type "Float (double-precision)") (TriggeredSeconds :type "Float (double-precision)") (InputAction :type "InputAction Object Reference" :default "/Game/MyContent/Player/Input/IA_AnyKey.IA_AnyKey"))
  (:`Triggered`
    (`/Game/MyContent/Player/BP_Player.OnAnyKeyPressed` (`self.PlayerRef`))))

(event `EnhancedInput|/Game/MyContent/Player/Input/IA_Mouse`
  (params (ActionValue :type Boolean) (ElapsedSeconds :type "Float (double-precision)") (TriggeredSeconds :type "Float (double-precision)") (InputAction :type "InputAction Object Reference" :default "/Game/MyContent/Player/Input/IA_Mouse.IA_Mouse")))

(event `EnhancedInput|/Game/MyContent/Player/Input/IA_Gamepad`
  (params (ActionValue :type Boolean) (ElapsedSeconds :type "Float (double-precision)") (TriggeredSeconds :type "Float (double-precision)") (InputAction :type "InputAction Object Reference" :default "/Game/MyContent/Player/Input/IA_Gamepad.IA_Gamepad")))

(fn `CreateWidgetRefs`
  (bind _returnvalue (`|CreateWidget` "/Game/MyContent/Menu/BP_UI_MainMenu.BP_UI_MainMenu_C"))
  (set `/Game/MyContent/Player/BP_Player.MainMenuRef` _returnvalue (`self.PlayerRef`))
  (bind _returnvalue_2 (`|CreateWidget` "/Game/MyContent/Menu/BP_UI_PauseMenu.BP_UI_PauseMenu_C"))
  (set `/Game/MyContent/Player/BP_Player.PauseMenuRef` _returnvalue_2 (`self.PlayerRef`))
  (bind _returnvalue_3 (`|CreateWidget` "/Game/MyContent/Menu/BP_UI_Chapters.BP_UI_Chapters_C"))
  (set `/Game/MyContent/Player/BP_Player.ChapterMenuRef` _returnvalue_3 (`self.PlayerRef`)))

(fn `DefaultInputs`
  (for _array_element (`|MakeArray` "/Game/MyContent/Player/Input/IMC_Default.IMC_Default" :!type "InputMappingContext Object Reference")
    (`EnhancedInputSubsystemInterface.AddMappingContext` (subsystem `EnhancedInputLocalPlayerSubsystem`) _array_element 0 (struct))))

(fn `UserConstructionScript`)