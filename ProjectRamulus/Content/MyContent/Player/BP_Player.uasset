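; BP_Player is the player Blueprint that holds narrative progress: current chapter, highest chapter, dialogue position and active widget index.
; Setter functions update these values and fire change events, keeping previous dialogue and widget indices; dialogue changes only notify from 2 upward.
; It registers itself with BP_GameInstance on possession and shows the mouse cursor on BeginPlay.
; It also resets defaults and toggles the pause menu outside the main menu.
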(event `self.ReceiveTick`
  (params (DeltaSeconds :type "Float (single-precision)")))

(event `self.ReceivePossessed`
  (params (NewController :type "Controller Object Reference"))
  (bind _asbp_game_instance (cast `/Game/MyContent/Core/BP_GameInstance` (`GameplayStatics.GetGameInstance`)))
  (set `/Game/MyContent/Core/BP_GameInstance.PlayerRef` self _asbp_game_instance))

(event `self.ReceiveBeginPlay`
  (bind _asbp_player_controller (cast `/Game/MyContent/Player/BP_PlayerController` (`GameplayStatics.GetPlayerController` 0)))
  (bind _output_get (set `self.PlayerControllerRef` _asbp_player_controller))
  (set `PlayerController.bShowMouseCursor` true _output_get))

(fn `PauseMenu`
  (if (not (`Widget.IsInViewport` (`self.MainMenuRef`)))
    (if (not (`Widget.IsInViewport` (`self.PauseMenuRef`)))
      (`GameplayStatics.SetGamePaused` true)
      (`UserWidget.AddToViewport` (`self.PauseMenuRef`) 1)
      (if (`self.DebugMode`)
        (`KismetSystemLibrary.PrintString` "Pause"))
      (else
        (`GameplayStatics.SetGamePaused` false)
        (`Widget.RemoveFromParent` (`self.PauseMenuRef`))
        (if (`self.DebugMode`)
          (`KismetSystemLibrary.PrintString` "Unpause"))))))

(fn `SetActiveWidget`
  (params (Index :type Integer))
  (set `self.LastActiveIndex` (`self.ActiveWidgetIndex`))
  (bind _output_get (set `self.ActiveWidgetIndex` (`local.Index`)))
  (`self.OnActiveWidgetChanged` _output_get))

(fn `SetChapter`
  (params (Chapter :type Integer))
  ; Actual chapter you are on
  (set `self.Chapter` Chapter)
  (`self.OnChapterChanged`))

(fn `SetDefaults`
  (`self.SetChapter` 0)
  (`self.SetDialogue` 0)
  (`self.SetActiveWidget` 0)
  (`self.SetMaxChapter` 0)
  (set `self.LastDialogue` 0)
  (if (`self.DebugMode`)
    (`KismetSystemLibrary.PrintString` "Defaults")))

(fn `SetDialogue`
  (params (Amount :type Integer))
  (set `self.LastDialogue` (`self.Dialogue`))
  (bind _output_get (set `self.Dialogue` (`KismetMathLibrary.Max` Amount)))
  (if (not (< _output_get 2))
    (`self.OnDialogueChanged`)
    (if (`self.DebugMode`)
      (`KismetSystemLibrary.PrintString` (`KismetTextLibrary.Conv_TextToString` (`|FormatText` "Dialogue {amount}" (`self.Dialogue`))) true true (struct :`R` 0.362739 :`G` 1.0 :`A` 1.0) 1.0))))

(fn `SetLastDialogue`
  (params (LastDialogue :type Integer))
  (set `self.LastDialogue` LastDialogue))

(fn `SetMaxChapter`
  (params (ChapterMax :type Integer))
  (set `self.ChapterMax` ChapterMax)
  (`self.OnMaxChapterChanged`))

(fn `UnlockNextChapter`
  (`self.SetMaxChapter` (+ (`self.ChapterMax`) 1))
  (`self.OnMaxChapterChanged`))

(fn `UserConstructionScript`)